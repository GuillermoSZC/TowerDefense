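; BP_GameMode is a game mode that grants loot directly to the player's hero.
; SpawnLoot looks up the requested item's enum name as a row in the supplied loot table, then adds one to player 0's BP_Hero using that row's Name.
; One enum value instead calls DetermineLoot for random selection by category, but that function is an unimplemented stub.
; BeginPlay, Tick and the construction script are empty.
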(fn `DetermineLoot`
  (params (Category :type "GameplayTag Structure"))
  (return))

(fn `SpawnLoot`
  (params (LootCategory :type "GameplayTag Structure") (LootItem :type "/Game/Logic/LootTables/Enumerators/E_LootItems Enum" :default "NewEnumerator0") (LootTable :type "DataTable Object Reference"))
  (bind _returnvalue (`KismetStringLibrary.Conv_StringToName` (`|GetEnumeratorNameAsString` LootItem)))
  (if (`|EnumEquality` LootItem "NewEnumerator12")
    ;[1 1 1] //TODO Select Random Loot from Category
    (`self.DetermineLoot` LootCategory)
    (else
      (bind _returnvalue_2 (`|GetDataTableRow` LootTable _returnvalue)
        (:`then`
          _))))
  (set `self.LocalDeterminedLoot` _returnvalue)
  (bind _asbp_hero (cast `/Game/GameFiles/Characters/Hero/BP_Hero` (`GameplayStatics.GetPlayerPawn` 0)))
  (`/Game/GameFiles/Characters/Hero/BP_Hero.AddLoot` _asbp_hero (`.Name_10_9F4D1C3C4FD240674C0E22ADB17C14D3` (break `/Game/Logic/LootTables/Structures/S_LootItems` _returnvalue_2)) 1)
  (return))

(fn `UserConstructionScript`)