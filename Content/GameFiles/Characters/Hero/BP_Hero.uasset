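; BP_Hero is the hero character Blueprint, holding a player inventory and setting up its element and ability system.
; BeginPlay resets the spawned element, initializes stats from TDLevelAttributeSet and applies the GE_LevelUp gameplay effect, while element changes defer to the parent.
; AddLoot increments only items already present in the inventory map.
; A debug Z key sets every existing inventory entry to a huge amount.
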(event EventBeginPlay
  (Class|TDElementComponent|TDSetSpawnedElement (Variables|Default|GetelementComponent) "None")
  (Class|AbilitySystemComponent|InitStats (Variables|Default|GetabilitySystem) "/Script/TowerDefense.TDLevelAttributeSet")
  (GameplayEffects|ApplyGameplayEffectToSelf :self (Variables|Default|GetabilitySystem) :GameplayEffectClass "/Game/GameFiles/Gas/GameplayEffect/GE_LevelUp.GE_LevelUp_C"))

(event EventTDonElementChange
  (params (_newElement :type EElements%20Enum :default "None"))
  (|CallParentFunction _newElement))

(event Input|KeyboardEvents|DebugKeyZ
  (params (Key :type Key%20Structure :default "None") (ActionValue :type Input%20Action%20Value%20Structure))
  (bind _playerinventory (Variables|Default|GetPlayerInventory))
  (:Pressed
    (bind _keys (Utilities|Map|Keys _playerinventory))
    (for _array_element _keys
      (Utilities|Map|Add _playerinventory _array_element 999999999))))

(fn ConstructionScript)

(fn AddLoot
  (params (LootItem :type ELootItems%20Enum :default "None") (Ammount :type Integer))
  (bind _playerinventory (Variables|Default|GetPlayerInventory))
  (bind (_value _returnvalue) (Utilities|Map|Find _playerinventory LootItem))
  (if _returnvalue
    (Utilities|Map|Add (Variables|Default|GetPlayerInventory) LootItem (+ Ammount _value))
    (return)))