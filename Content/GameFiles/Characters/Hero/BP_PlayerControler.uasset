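; Player controller Blueprint that adds debug cheat keys for controlling round timing.
; A Cheats graph binds debug keys that call the round manager: M and N pause and resume time, while J and K lengthen and shorten the buy phase by a fixed step.
; BeginPlay only calls the parent implementation, and the construction script is empty.
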(event EventBeginPlay
  (|CallParentFunction))

(event Input|KeyboardEvents|DebugKeyK
  (params (Key :type Key%20Structure :default "None") (ActionValue :type Input%20Action%20Value%20Structure))
  (:Pressed
    (Class|TDRoundManager|TDModifyBuyPhaseTime (Class|TDGameData|TDGetRoundManager) -5.0)))

(event Input|KeyboardEvents|DebugKeyM
  (params (Key :type Key%20Structure :default "None") (ActionValue :type Input%20Action%20Value%20Structure))
  (:Pressed
    (Class|TDRoundManager|TDSetTimePaused (Class|TDGameData|TDGetRoundManager) true)))

(event Input|KeyboardEvents|DebugKeyN
  (params (Key :type Key%20Structure :default "None") (ActionValue :type Input%20Action%20Value%20Structure))
  (:Pressed
    (Class|TDRoundManager|TDSetTimePaused (Class|TDGameData|TDGetRoundManager) false)))

(event Input|KeyboardEvents|DebugKeyJ
  (params (Key :type Key%20Structure :default "None") (ActionValue :type Input%20Action%20Value%20Structure))
  (:Pressed
    (Class|TDRoundManager|TDModifyBuyPhaseTime (Class|TDGameData|TDGetRoundManager) 5.0)))

(fn ConstructionScript)