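; Lich enemy spell projectile that homes in on the player, then flies straight, with a timed self-destruct.
; On spawn, a timeline lerps the sphere from its start toward the player's live position while facing them.
; When the timeline finishes, Tick is enabled to move the actor forward at Velocity.
; Any overlap destroys it; targets with an ability system trigger a hit sound and receive the owner's GAS damage effect.
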(event `CustomEvent`
  (`self.K2_DestroyActor`))

(event `self.ReceiveBeginPlay`
  (bind _returnvalue (`self.K2_GetActorLocation` (`TDGameData.TDGetPlayerRef`)))
  (`KismetSystemLibrary.K2_SetTimerDelegate` (delegate `CustomEvent`) 10.0)
  (`self.SetActorTickEnabled` false)
  (set `self.StartPos` (`self.K2_GetActorLocation`))
  (bind (_direction _newtrack_0) (`Timeline|Timeline` :!via `PlayFromStart`)
    (:`Update`
      (`SceneComponent.K2_SetWorldLocationAndRotation` (`self.Sphere1`) (`KismetMathLibrary.VLerp` (`self.StartPos`) _returnvalue _newtrack_0) (`KismetMathLibrary.FindLookAtRotation` (`self.K2_GetActorLocation`) _returnvalue) false false))
    (:`Finished`
      (`self.SetActorTickEnabled` true))))

(event `self.ReceiveTick`
  (params (DeltaSeconds :type "Float (single-precision)"))
  (`self.K2_SetActorLocation` (+ (`self.K2_GetActorLocation`) (* (* (`self.GetActorForwardVector`) (`self.Velocity`)) DeltaSeconds))))

(event `self.Sphere1.OnComponentBeginOverlap`
  (params (OverlappedComponent :type "PrimitiveComponent Object Reference") (OtherActor :type "Actor Object Reference") (OtherComp :type "PrimitiveComponent Object Reference") (OtherBodyIndex :type Integer) (bFromSweep :type Boolean) (SweepResult :type "HitResult Structure (by ref)"))
  (bind _returnvalue (`AbilitySystemBlueprintLibrary.GetAbilitySystemComponent` OtherActor))
  (bind _ownerasc (`self.OwnerASC`))
  (`/Engine/EditorBlueprintResources/StandardMacros.IsValid` _returnvalue
    (:`Is Valid`
      (`GameplayStatics.SpawnSoundAtLocation` "/Game/GameFiles/SFX/MetaSounds/MS_LichHit.MS_LichHit" (`self.K2_GetActorLocation`) (struct) 1.0 1.0 0.0 null null)
      (`/Engine/EditorBlueprintResources/StandardMacros.IsValid` _ownerasc
        (:`Is Valid`
          (`AbilitySystemComponent.BP_ApplyGameplayEffectToTarget` :`self` _ownerasc :`GameplayEffectClass` "/Game/GameFiles/Gas/GameplayEffect/GE_DamageLichSpell.GE_DamageLichSpell_C" :`Target` _returnvalue))
        (:`Is Not Valid`
          _)))
    (:`Is Not Valid`
      _))
  (`self.K2_DestroyActor`))

(fn `UserConstructionScript`)