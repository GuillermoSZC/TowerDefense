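; BP_BalisticTower is a ballistic tower Blueprint that aims its head and fires through the Gameplay Ability System.
; TDRotateHeadTower calls the parent, then turns the Sphere component toward the target position using a 2D-normalized direction, with no sweep.
; TGGApplyEffect overrides the parent without calling it, sending itself an Ability.trigger.shoot gameplay event with the tower's ability struct as optional payload.
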(event `TDInterface.TDRotateHeadTower`
  (params (_PositionToLook :type "Vector Structure (by ref)"))
  (bind _sphere (`self.Sphere`))
  (`parent.TDRotateHeadTower` _PositionToLook)
  (`SceneComponent.K2_SetWorldRotation` _sphere (`KismetMathLibrary.Quat_Rotator` (`KismetMathLibrary.Conv_VectorToQuaternion` (`KismetMathLibrary.Vector_Normal2D` (- _PositionToLook (`SceneComponent.K2_GetComponentLocation` _sphere))))) false false))

(fn `TGGApplyEffect`
  (returns (ReturnValue :type Integer))
  (`AbilitySystemBlueprintLibrary.SendGameplayEventToActor` self (struct :`TagName` "ability.trigger.shoot") (make `GameplayEventData` (struct) null null (`TDGameData.TDGetAbilityStrcut`)))
  (return 0))

(fn `UserConstructionScript`)