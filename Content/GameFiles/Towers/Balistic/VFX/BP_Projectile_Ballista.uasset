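; Ballista tower projectile that flies to an assigned enemy and delivers a Gameplay Effect on arrival.
; SetEnemyPosition supplies the target actor, instigator and effect spec.
; From BeginPlay, a timeline lerps it without sweep from its spawn point to the enemy's live location, so it homes without collision.
; When the timeline finishes, it applies the spec through the instigator's Ability System Component, spawns an impact actor at the enemy and destroys itself.
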(event `self.ReceiveBeginPlay`
  (bind _enemyposition (`self.EnemyPosition`))
  (set `self.IntiialPosition` (`self.K2_GetActorLocation`))
  (bind (_direction _newtrack_0) (`Timeline|BulletLocation` :!via `PlayFromStart`)
    (:`Update`
      (`/Engine/EditorBlueprintResources/StandardMacros.IsValid` _enemyposition
        (:`Is Valid`
          (`self.K2_SetActorLocation` (`KismetMathLibrary.VLerp` (`self.IntiialPosition`) (`self.K2_GetActorLocation` _enemyposition) _newtrack_0)))))
    (:`Finished`
      (`AbilitySystemComponent.BP_ApplyGameplayEffectSpecToTarget` (`AbilitySystemBlueprintLibrary.GetAbilitySystemComponent` (`self.ActorInstigator`)) (`self.GE`) (`AbilitySystemBlueprintLibrary.GetAbilitySystemComponent` (`self.EnemyPosition`)))
      (`|SpawnActorFromClass` (`self.ImpactActor`) (`KismetMathLibrary.MakeTransform` (`self.K2_GetActorLocation` (`self.EnemyPosition`))) "Undefined" "OverrideRootScale" null null)
      (`self.K2_DestroyActor`))))

(fn `Set enemy position`
  (params (EnemyReference :type "Actor Object Reference") (OwnerRef :type "Actor Object Reference") (`GE To apply` :type "GameplayEffectSpecHandle Structure"))
  (set `self.EnemyPosition` EnemyReference)
  (set `self.ActorInstigator` OwnerRef)
  (set `self.GE` `GE To apply`))

(fn `UserConstructionScript`)