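; BP_SphereArea is a tower sphere area actor pairing a collision sphere with a visible, element-colored volume.
; On BeginPlay, the Normal and InverseNormal meshes share one dynamic material instance.
; SetSphereRadius resizes the collision and scales both meshes to match, assuming a 50-unit base radius.
; ChangeElement looks up the element in ColorMap and applies that color to both material color parameters.
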(event `self.ReceiveBeginPlay`
  (bind _normal (`self.Normal`))
  (bind _returnvalue (`PrimitiveComponent.CreateDynamicMaterialInstance` _normal 0 (`PrimitiveComponent.GetMaterial` _normal 0) "None"))
  (bind _output_get (set `self.DynamicMaterial` _returnvalue))
  (`PrimitiveComponent.SetMaterial` (`self.Normal`) 0 _output_get)
  (`PrimitiveComponent.SetMaterial` (`self.InverseNormal`) 0 _output_get))

(fn `ChangeElement`
  (params (EElement :type "EElements Enum" :default "None"))
  (bind _dynamicmaterial (`self.DynamicMaterial`))
  (bind (_value _returnvalue) (`BlueprintMapLibrary.Map_Find` (`self.ColorMap`) EElement))
  (if _returnvalue
    (`MaterialInstanceDynamic.SetVectorParameterValue` _dynamicmaterial "Color_01" _value)
    (`MaterialInstanceDynamic.SetVectorParameterValue` _dynamicmaterial "Color_02" _value)))

(fn `SetSphereRadius`
  (params (Radius :type "Float (double-precision)"))
  (bind _returnvalue (/ Radius 50.0))
  (bind _returnvalue_2 (`KismetMathLibrary.MakeVector` _returnvalue _returnvalue _returnvalue))
  (`SphereComponent.SetSphereRadius` (`self.SphereCollision`) Radius true)
  (`SceneComponent.SetRelativeScale3D` (`self.Normal`) _returnvalue_2)
  (`SceneComponent.SetRelativeScale3D` (`self.InverseNormal`) _returnvalue_2))

(fn `UserConstructionScript`)