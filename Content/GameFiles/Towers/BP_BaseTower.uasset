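; Base tower actor for the tower defense game, with an element component and a Gameplay Ability System component.
; On BeginPlay it sets the None element, initializes stats from the level attribute set and applies GE_LevelUp to itself at level zero.
; A debug helper checks whether a "TD.ShowDebug"-prefixed console variable equals one.
; The head rotation event is an empty stub, and there is no active tick or overlap logic.
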(event `self.ReceiveBeginPlay`
  (`TDElementComponent.TDSetSpawnedElement` (`self.elementComponent`) "/Game/GameFiles/Elements/DA_NoneElement.DA_NoneElement")
  (`AbilitySystemComponent.K2_InitStats` (`self.abilitySystem`) "/Script/TowerDefense.TDLevelAttributeSet" null)
  (`AbilitySystemComponent.BP_ApplyGameplayEffectToSelf` :`self` (`self.abilitySystem`) :`GameplayEffectClass` "/Game/GameFiles/Gas/GameplayEffect/GE_LevelUp.GE_LevelUp_C"))

(event `TDInterface.TDRotateHeadTower`
  (params (_PositionToLook :type "Vector Structure (by ref)")))

(fn `TDIsDebugActive`
  (returns (ReturnValue :type Boolean))
  (bind _returnvalue (`KismetSystemLibrary.GetConsoleVariableIntValue` (`KismetStringLibrary.Concat_StrStr` "TD.ShowDebug" (`self.ConsoleVariable`))))
  (return (== _returnvalue 1)))

(fn `UserConstructionScript`)