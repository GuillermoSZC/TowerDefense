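; Sonic tower Blueprint: a tower with a radar dish that turns toward its target and fires through the Gameplay Ability System.
; Head rotation extends the parent's, turning the radar neck along the horizontal direction to the look position and storing it in HeadRotation.
; TGGApplyEffect replaces the parent logic with a shoot gameplay event sent to itself.
; Shot position and rotation come from the head's SonicRay socket; NiagaraFX spawns three attached effects.
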(event `TDInterface.TDRotateHeadTower`
  (params (_PositionToLook :type "Vector Structure (by ref)"))
  (bind _sonictower_tower_radarneck (`self.sonictower_Tower_RadarNeck`))
  (bind _returnvalue (`KismetMathLibrary.Conv_VectorToQuaternion` (`KismetMathLibrary.Vector_Normal2D` (- _PositionToLook (`SceneComponent.K2_GetComponentLocation` _sonictower_tower_radarneck)))))
  (`parent.TDRotateHeadTower` _PositionToLook)
  (`SceneComponent.K2_SetWorldRotation` _sonictower_tower_radarneck (`KismetMathLibrary.Quat_Rotator` _returnvalue) false false)
  (set `self.HeadRotation ` _returnvalue))

(fn `NiagaraFX`
  (`NiagaraFunctionLibrary.SpawnSystemAttached` null null "None" (0.0 0.0 0.0) (struct) "KeepRelativeOffset")
  (`NiagaraFunctionLibrary.SpawnSystemAttached` null null "None" (0.0 0.0 0.0) (struct) "KeepRelativeOffset")
  (`NiagaraFunctionLibrary.SpawnSystemAttached` null null "None" (0.0 0.0 0.0) (struct) "KeepRelativeOffset"))

(fn `TDGetShootPosition`
  (returns (ReturnValue :type "Vector Structure"))
  (return (`SceneComponent.GetSocketLocation` (`self.sonictower_Tower_RadarHead`) "SonicRay")))

(fn `TDGetShootRotation`
  (returns (ReturnValue :type "Rotator Structure"))
  (return (`SceneComponent.GetSocketRotation` (`self.sonictower_Tower_RadarHead`) "SonicRay")))

(fn `TGGApplyEffect`
  (returns (ReturnValue :type Integer))
  (`AbilitySystemBlueprintLibrary.SendGameplayEventToActor` self (struct :`TagName` "ability.trigger.shoot") (make `GameplayEventData` (struct) null null (`TDGameData.TDGetAbilityStrcut`)))
  (return 0))

(fn `UserConstructionScript`)